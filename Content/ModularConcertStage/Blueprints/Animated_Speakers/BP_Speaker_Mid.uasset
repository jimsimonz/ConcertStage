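; BP_Speaker_Mid is an animated mid speaker for the modular concert stage, driven by a Speed variable.
; On BeginPlay it stores Speed as Startspeed and overrides the skeletal mesh's animation data to play SK_Speaker_Mid_Anim at that rate.
; Tick compares Speed with Startspeed and calls PlayRateChange on a mismatch, which reruns that same setup with the new rate.
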(event Custom|PlayRateChange
  (Variables|Default|SetStartspeed (Variables|Default|GetSpeed))
  (Components|Animation|OverrideAnimationData (Variables|Default|GetSK_Speaker_Mid) "/ConcertStage/ModularConcertStage/Meshes/Speakers_Rigged/SK_Speaker_Mid_Anim.SK_Speaker_Mid_Anim" true true 0.0 (Variables|Default|GetSpeed)))

(event EventBeginPlay
  (Variables|Default|SetStartspeed (Variables|Default|GetSpeed))
  (Components|Animation|OverrideAnimationData (Variables|Default|GetSK_Speaker_Mid) "/ConcertStage/ModularConcertStage/Meshes/Speakers_Rigged/SK_Speaker_Mid_Anim.SK_Speaker_Mid_Anim" true true 0.0 (Variables|Default|GetSpeed)))

(event Collision|EventActorBeginOverlap
  (params (OtherActor :type Actor%20Object%20Reference)))

(event EventTick
  (params (DeltaSeconds :type Float%20%28single-precision%29))
  (if (not (== (Variables|Default|GetSpeed) (Variables|Default|GetStartspeed)))
    (CallFunction|PlayRateChange)))

(fn ConstructionScript)
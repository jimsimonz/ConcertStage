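; BP_Light_Par_Can is a configurable par can lamp for the modular concert stage, set up entirely in its construction script.
; Exposed rotation values yaw the hanger and pitch the lamp body.
; Color and intensity drive both the spot light and a dynamic emissive material on the lamp mesh, with intensity scaled down for the material.
; Beam intensity sets the spot light's volumetric scattering, and the event graph holds no active logic.
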(event EventBeginPlay)

(event Collision|EventActorBeginOverlap
  (params (OtherActor :type Actor%20Object%20Reference)))

(event EventTick
  (params (DeltaSeconds :type Float%20%28single-precision%29)))

(fn ConstructionScript
  (bind _light_intensity (Variables|Default|GetLight_Intensity))
  (bind _spotlight (Variables|Default|GetSpotLight))
  (bind _sm_par_can_light (Variables|Default|GetSM_Par_Can_Light))
  (bind _light_color (Variables|Default|GetLight_Color))
  (Transformation|SetRelativeRotation (Variables|Default|GetSM_Par_Can_Hanger) (Math|Rotator|MakeRotator 0.0 0.0 (Variables|Default|GetVertical_Rotation)) false false)
  (Transformation|SetRelativeRotation _sm_par_can_light (Math|Rotator|MakeRotator 0.0 (Variables|Default|GetHorizontal_Rotation%20%28Up%20and%20Down%29) 0.0) false false)
  (bind _returnvalue (Rendering|Material|CreateDynamicMaterialInstance _sm_par_can_light 1 "/ConcertStage/ModularConcertStage/Materials/Instances/MI_Light_Emissive_Par_Can.MI_Light_Emissive_Par_Can" "None" :!class /Script/Engine.PrimitiveComponent))
  (Rendering|Material|SetVectorParameterValue _returnvalue "Light_Color" _light_color :!class /Script/Engine.MaterialInstanceDynamic)
  (Rendering|Material|SetScalarParameterValue _returnvalue "Light_Emissive_Intensity" (/ _light_intensity 1e+03) :!class /Script/Engine.MaterialInstanceDynamic)
  (Rendering|Components|Light|SetLightColor _spotlight _light_color true)
  (Rendering|Components|Light|SetIntensity _spotlight _light_intensity)
  (Class|LightComponent|SetVolumetricScatteringIntensity _spotlight (Variables|Default|GetLight%20Beam%20Intensity)))